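; BP_Lever is a switchable lever actor that runs a 15-second cooldown when activated and shows its on or off state.
; Activate calls the game instance's timer sound update, restarts the countdown and shows the ON component.
; A looping one-second timer decrements the cooldown and writes it to BP_GameInstance, from which BeginPlay also restores it.
; Tick watches that shared value and flips back to OFF at zero through a DoOnce that Activate re-arms.
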(event Custom|UpdateObject
  (bind _output_get (Variables|Default|SetCooldown (Math|Integer|Clamp(Integer) (- (Variables|Default|GetCooldown) 1) 0 15)))
  (Variables|/Game/Game/Blueprint/GameInstance/BP_GameInstance.BP_GameInstance_C|SetCooldown (Variables|Default|GetAs%20BP%20Game%20Instance) _output_get))

(event EventBeginPlay
  (bind _asbp_game_instance (Utilities|Casting|CastToBP_GameInstance (Game|GetGameInstance)))
  (bind _output_get (Variables|Default|SetAs%20BP%20Game%20Instance _asbp_game_instance))
  (Variables|Default|SetCooldown (Variables|/Game/Game/Blueprint/GameInstance/BP_GameInstance.BP_GameInstance_C|GetCooldown _output_get))
  (bind _returnvalue (Utilities|Time|SetTimerbyEvent (delegate Custom|UpdateObject) 1.0 true))
  (Variables|Default|SetTimer _returnvalue))

(event Collision|EventActorBeginOverlap
  (params (OtherActor :type Actor%20Object%20Reference)))

(event EventTick
  (params (DeltaSeconds :type Float%20%28single-precision%29))
  (if (not (> (Variables|/Game/Game/Blueprint/GameInstance/BP_GameInstance.BP_GameInstance_C|GetCooldown (Variables|Default|GetAs%20BP%20Game%20Instance)) 0))
    (Utilities|FlowControl|DoOnce false
      (:Completed
        (Rendering|SetVisibility (Variables|Default|GetSwitchOFF) true false)
        (Rendering|SetVisibility (Variables|Default|GetSwitchON) false false)))))

(event EventActivate
  (Default|UpdateTimerSound (Variables|Default|GetAs%20BP%20Game%20Instance))
  (Variables|Default|SetCooldown 15)
  (Rendering|SetVisibility (Variables|Default|GetSwitchOFF) false false)
  (Rendering|SetVisibility (Variables|Default|GetSwitchON) true false)
  (Utilities|FlowControl|DoOnce false) ; enters at Reset
)

(fn ConstructionScript)