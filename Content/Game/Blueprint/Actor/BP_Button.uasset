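; BP_Button is a button actor that, when activated, updates the state of its controlled door through the game instance.
; BeginPlay caches the cube's starting scale and the BP_GameInstance reference.
; Activate passes DoorControlled to the game instance's UpdateDoorState and switches the cube to a green material.
; A FlipFlop-driven timeline for squeezing the cube's scale is present but unconnected, so it never runs.
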(event EventBeginPlay
  (Variables|Default|SetRelative%20Scale%203D (Variables|/Script/Engine.SceneComponent|GetRelativeScale3D (Variables|Default|GetCube)))
  (bind _asbp_game_instance (Utilities|Casting|CastToBP_GameInstance (Game|GetGameInstance)))
  (Variables|Default|SetAs%20BP%20Game%20Instance _asbp_game_instance))

(event Collision|EventActorBeginOverlap
  (params (OtherActor :type Actor%20Object%20Reference)))

(event EventTick
  (params (DeltaSeconds :type Float%20%28single-precision%29)))

(event EventActivate
  (Default|UpdateDoorState (Variables|Default|GetAs%20BP%20Game%20Instance) (Variables|Default|GetDoorControlled))
  (Rendering|Material|SetMaterial (Variables|Default|GetCube) 0 "/AnimationSharing/AnimSharingGreen.AnimSharingGreen"))

(fn ConstructionScript)