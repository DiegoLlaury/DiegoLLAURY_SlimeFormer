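; BP_Door is a door actor that lowers its cube to open when the game instance signals a door state change.
; On BeginPlay it binds UpdateDoor to BP_GameInstance's DoorState event, which plays a timeline if InteractDoor returns true.
; Each timeline update lerps from the cube's current world location toward 120 units below, applied as relative location.
; Button binding is unwired, and ButtonChange and OpenDoor are empty.
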(event Custom|OpenDoor
  (params (Player :type Actor%20Object%20Reference)))

(event Custom|ButtonChange)

(event Custom|UpdateDoor
  (bind _cube (Variables|Default|GetCube))
  (bind _returnvalue (Transformation|GetWorldLocation _cube))
  (bind _returnvalue_2 (Default|InteractDoor (stale EventBeginPlay _output_get)))
  (if _returnvalue_2
    (bind _opentrack (Timeline|OpenDoorT Play)
      (:Update
        (Transformation|SetRelativeLocation (Variables|Default|GetCube) (Math|Vector|Lerp(Vector) _returnvalue (- _returnvalue "0.000000,0.000000,120.000000") _opentrack) false false)))))

(event EventBeginPlay
  (bind _asbp_game_instance (Utilities|Casting|CastToBP_GameInstance (Game|GetGameInstance)))
  (bind _output_get (Variables|Default|SetAs%20BP%20Game%20Instance _asbp_game_instance))
  (EventDispatchers|BindEventtoDoorState _output_get (delegate Custom|UpdateDoor)))

(event Collision|EventActorBeginOverlap
  (params (OtherActor :type Actor%20Object%20Reference)))

(event EventTick
  (params (DeltaSeconds :type Float%20%28single-precision%29)))

(fn ConstructionScript)